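; Blueprint function library of shared helpers for fetching the game's core framework objects and printing debug messages.
; GetGameInstance and GetGameMode return the current objects cast to BP_GameInstance and BP_Gamemode, printing a red on-screen error if the cast fails.
; DebugPrint prints only when the game instance's DebugPrint flag is on, prefixing each message with the calling object's name.
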(fn `DebugPrint`
  (params (InString :type String :default "Hello") (`Print to Screen` :type Boolean :default true) (`Print to Log` :type Boolean :default true) (TexrColor :type "LinearColor Structure" :default (struct :`R` 1.0 :`A` 1.0)) (Duration :type "Float (double-precision)" :default 2.0) (Key :type Name :default "None") (SelfRef :type "Object Object Reference"))
  (if (`/Game/Blueprints/System/BP_GameInstance.bDebugPrint` (`self.GetGameInstance` null))
    (`KismetSystemLibrary.PrintString` null (`KismetStringLibrary.Concat_StrStr` "[ " (`KismetSystemLibrary.GetObjectName` SelfRef) " ] : " InString) `Print to Screen` `Print to Log` TexrColor Duration Key)))

(fn `GetGameInstance`
  (returns (GameInstance :type "/Game/Blueprints/System/BP_GameInstance Object Reference"))
  (bind _asbp_game_instance (cast `/Game/Blueprints/System/BP_GameInstance` (`GameplayStatics.GetGameInstance` null))
    (:`then`
      (return _asbp_game_instance))
    (:`CastFailed`
      (`KismetSystemLibrary.PrintString` null "Error : Failed to cast BP_GameInstance!" true false (struct :`R` 1.0 :`A` 1.0))
      (return null))))

(fn `GetGameMode`
  (returns (GameMode :type "/Game/Blueprints/System/BP_Gamemode Object Reference"))
  (bind _asbp_gamemode (cast `/Game/Blueprints/System/BP_Gamemode` (`GameplayStatics.GetGameMode` null))
    (:`then`
      (return _asbp_gamemode))
    (:`CastFailed`
      (`KismetSystemLibrary.PrintString` null "Error : Failed to cast BP_GameMode!" true false (struct :`R` 1.0 :`A` 1.0))
      (return null))))