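; BP_Debris is a moving actor that feeds object and position data to Niagara debris effects, apparently as a test setup.
; BeginPlay passes itself to a referenced Niagara actor, then after a delay activates NSDebrisB and fills its position array with random points near the actor.
; Tick nudges the actor along world X every frame, without sweep.
; A disconnected FlipFlop chain for kill-and-respawn with alternating spawn counts never runs, and ParticleData is empty.
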(event `self.ReceiveBeginPlay`
  (bind _ns_debrisb (`self.NS_DebrisB`))
  (`NiagaraComponent.SetVariableObject` (`NiagaraActor.NiagaraComponent` (`self.RefActorNSA`)) "RefActor" self)
  (`KismetSystemLibrary.Delay` 1.0)
  (`ActorComponent.Activate` _ns_debrisb false)
  (for _ (range 100)
    (`KismetArrayLibrary.Array_Add` (`self.position`) (+ (`self.K2_GetActorLocation`) (`KismetMathLibrary.MakeVector` (`KismetMathLibrary.RandomFloatInRange` 0.0 100.0) (`KismetMathLibrary.RandomFloatInRange` 0.0 100.0) (`KismetMathLibrary.RandomFloatInRange` 0.0 100.0)))))
  (`NiagaraDataInterfaceArrayFunctionLibrary.SetNiagaraArrayPosition` _ns_debrisb "PositionArrays" (`self.position`)))

(event `self.ReceiveTick`
  (params (DeltaSeconds :type "Float (single-precision)"))
  (`self.K2_AddActorWorldOffset` (1.0 0.0 0.0)))

(event `self.ReceiveParticleData`
  (params (Data :type "Array of BasicParticleData Structure (by ref)") (NiagaraSystem :type "NiagaraSystem Object Reference") (SimulationPositionOffset :type "Vector Structure (by ref)")))

(fn `UserConstructionScript`)