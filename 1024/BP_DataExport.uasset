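; BP_DataExport is a debug Blueprint that receives particle data exported from Niagara and prints it on screen.
; Its construction script passes itself to the NSDataExport system as the RefActor object variable, making it the callback target.
; Two events each wait half a second, then print every particle's Size (labelled as ID), Position and Velocity.
; The custom receive variant also prints Age, in a distinct text color.
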(event `self.ReceiveParticleData`
  (params (Data :type "Array of BasicParticleData Structure (by ref)") (NiagaraSystem :type "NiagaraSystem Object Reference") (SimulationPositionOffset :type "Vector Structure (by ref)"))
  (`KismetSystemLibrary.Delay` 0.5)
  (for _array_element Data
    (bind (_position _size _velocity) (break `BasicParticleData` _array_element))
    (`KismetSystemLibrary.PrintString` (`KismetStringLibrary.Concat_StrStr` (`KismetStringLibrary.Concat_StrStr` "[ ID : " (`KismetStringLibrary.Conv_DoubleToString` _size)) (`KismetStringLibrary.Concat_StrStr` " ]  [ Pos : " (`KismetStringLibrary.Conv_VectorToString` _position)) (`KismetStringLibrary.Concat_StrStr` " ]  [ Vel : " (`KismetStringLibrary.Conv_VectorToString` _velocity) " ]")) true true (struct :`G` 0.66 :`B` 1.0 :`A` 1.0) 0.5)))

(event `self.CustomReceiveParticleData`
  (params (Data :type "Array of GgNDI_BasicParticleData Structure (by ref)") (NiagaraSystem :type "NiagaraSystem Object Reference") (SimulationPositionOffset :type "Vector Structure (by ref)"))
  (`KismetSystemLibrary.Delay` 0.5)
  (for _array_element Data
    (bind (_position _size _velocity _age) (break `GgNDI_BasicParticleData` _array_element))
    (`KismetSystemLibrary.PrintString` (`KismetStringLibrary.Concat_StrStr` (`KismetStringLibrary.Concat_StrStr` "[ ID : " (`KismetStringLibrary.Conv_DoubleToString` _size)) (`KismetStringLibrary.Concat_StrStr` " ]  [ Pos : " (`KismetStringLibrary.Conv_VectorToString` _position)) (`KismetStringLibrary.Concat_StrStr` " ]  [ Vel : " (`KismetStringLibrary.Conv_VectorToString` _velocity)) (`KismetStringLibrary.Concat_StrStr` " ]  [ Age : " (`KismetStringLibrary.Conv_DoubleToString` _age) " ]")) true true (struct :`R` 1.0 :`G` 0.5 :`B` 1.0 :`A` 1.0) 0.5)))

(fn `UserConstructionScript`
  (`NiagaraComponent.SetVariableObject` (`self.NS_DataExport`) "RefActor" self))