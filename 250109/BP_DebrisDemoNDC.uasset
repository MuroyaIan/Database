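; Demo Blueprint that writes test debris entries to the NDC_DebrisDemo Niagara Data Channel when play begins.
; It opens one two-entry write, visible to Blueprint and Niagara CPU and GPU, then fills Position, Normal and Surface per entry.
; Both entries share a position but have opposite vertical normals and different surface indices.
; Tick is empty, and two alternative write chains, one delayed, are left unconnected.
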(event `self.ReceiveBeginPlay`
  (bind _returnvalue (`NiagaraDataChannelLibrary.WriteToNiagaraDataChannel` "/Game/PRJ/VFX/NCD/NDC_DebrisDemo.NDC_DebrisDemo" (struct) 2 true true true))
  (`NiagaraDataChannelWriter.WritePosition` _returnvalue "Position" 0 (0.0 0.0 100.0))
  (`NiagaraDataChannelWriter.WritePosition` _returnvalue "Position" 0 (0.0 0.0 100.0))
  (`NiagaraDataChannelWriter.WriteVector` _returnvalue "Normal" 0 (0.0 0.0 1.0))
  (`NiagaraDataChannelWriter.WriteInt` _returnvalue "Surface" 0 0)
  (`NiagaraDataChannelWriter.WritePosition` _returnvalue "Position" 1 (0.0 0.0 100.0))
  (`NiagaraDataChannelWriter.WriteVector` _returnvalue "Normal" 1 (0.0 0.0 -1.0))
  (`NiagaraDataChannelWriter.WriteInt` _returnvalue "Surface" 1 1))

(event `self.ReceiveTick`
  (params (DeltaSeconds :type "Float (single-precision)")))

(fn `UserConstructionScript`)