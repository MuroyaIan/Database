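; Debris actor that hands particles between two Niagara systems, a 100-slot A and a 10-slot B, based on distance to itself.
; Particle data exported from Niagara moves nearby A particles into free B slots and returns them to their original slots once out of range.
; Usage and one-shot reset bool arrays are pushed back to Niagara, with mass, position, velocity and rotation carrying each particle's state across.
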(event `self.ReceiveBeginPlay`
  (bind _bparticleusageb (`self.bParticleUsageB`))
  (bind _bparticleresetb (`self.bParticleResetB`))
  (bind _bparticlereseta (`self.bParticleResetA`))
  (bind _ns_debrisb (`self.NS_DebrisB`))
  (bind _dummyf (`self.DummyF`))
  (bind _dummyv3 (`self.DummyV3`))
  (bind _dummyv4 (`self.DummyV4`))
  (bind _dummyf_2 (`self.DummyF`))
  (bind _dummyv3_2 (`self.DummyV3`))
  (bind _dummyv4_2 (`self.DummyV4`))
  (bind _bparticleusagea (`self.bParticleUsageA`))
  (bind _niagaracomponent (`NiagaraActor.NiagaraComponent` (`self.RefActorNSA`)))
  (`NiagaraComponent.SetVariableObject` (`NiagaraActor.NiagaraComponent` (`self.RefActorNSA`)) "RefActor" self)
  (`KismetArrayLibrary.Array_Resize` _bparticleusagea 100)
  (for (_ _array_index) _bparticleusagea
    (`KismetArrayLibrary.Array_Set` _bparticleusagea _array_index true))
  (`NiagaraDataInterfaceArrayFunctionLibrary.SetNiagaraArrayBool` (`NiagaraActor.NiagaraComponent` (`self.RefActorNSA`)) "UseParticle" _bparticleusagea)
  (`KismetArrayLibrary.Array_Resize` (`self.ParticleDataA`) 100)
  (`KismetArrayLibrary.Array_Resize` _bparticlereseta 100)
  (for (_ _array_index_2) _bparticlereseta
    (`KismetArrayLibrary.Array_Set` _bparticlereseta _array_index_2))
  (`NiagaraDataInterfaceArrayFunctionLibrary.SetNiagaraArrayBool` (`NiagaraActor.NiagaraComponent` (`self.RefActorNSA`)) "ResetParticle" _bparticlereseta)
  (`KismetArrayLibrary.Array_Resize` _dummyf_2 100)
  (`KismetArrayLibrary.Array_Resize` _dummyv3_2 100)
  (`KismetArrayLibrary.Array_Resize` _dummyv4_2 100)
  (`NiagaraDataInterfaceArrayFunctionLibrary.SetNiagaraArrayFloat` _niagaracomponent "InitMass" _dummyf_2)
  (`NiagaraDataInterfaceArrayFunctionLibrary.SetNiagaraArrayVector` _niagaracomponent "InitPos" _dummyv3_2)
  (`NiagaraDataInterfaceArrayFunctionLibrary.SetNiagaraArrayVector` _niagaracomponent "InitVel" _dummyv3_2)
  (`NiagaraDataInterfaceArrayFunctionLibrary.SetNiagaraArrayVector4` _niagaracomponent "InitRot" _dummyv4_2)
  (`NiagaraComponent.SetVariableObject` (`self.NS_DebrisB`) "RefActor" self)
  (`KismetArrayLibrary.Array_Resize` _bparticleusageb 10)
  (for (_ _array_index_3) _bparticleusageb
    (`KismetArrayLibrary.Array_Set` _bparticleusageb _array_index_3))
  (`NiagaraDataInterfaceArrayFunctionLibrary.SetNiagaraArrayBool` (`self.NS_DebrisB`) "UseParticle" _bparticleusageb)
  (`KismetArrayLibrary.Array_Resize` (`self.ParticleDataToB`) 10)
  (`KismetArrayLibrary.Array_Resize` _bparticleresetb 10)
  (for (_ _array_index_4) _bparticleresetb
    (`KismetArrayLibrary.Array_Set` _bparticleresetb _array_index_4))
  (`NiagaraDataInterfaceArrayFunctionLibrary.SetNiagaraArrayBool` (`self.NS_DebrisB`) "ResetParticle" _bparticleresetb)
  (`KismetArrayLibrary.Array_Resize` _dummyf 10)
  (`KismetArrayLibrary.Array_Resize` _dummyv3 10)
  (`KismetArrayLibrary.Array_Resize` _dummyv4 10)
  (`NiagaraDataInterfaceArrayFunctionLibrary.SetNiagaraArrayFloat` _ns_debrisb "InitMass" _dummyf)
  (`NiagaraDataInterfaceArrayFunctionLibrary.SetNiagaraArrayVector` _ns_debrisb "InitPos" _dummyv3)
  (`NiagaraDataInterfaceArrayFunctionLibrary.SetNiagaraArrayVector` _ns_debrisb "InitVel" _dummyv3)
  (`NiagaraDataInterfaceArrayFunctionLibrary.SetNiagaraArrayVector4` _ns_debrisb "InitRot" _dummyv4)
  (`KismetArrayLibrary.Array_Resize` (`self.DummyF`))
  (`KismetArrayLibrary.Array_Resize` (`self.DummyV3`))
  (`KismetArrayLibrary.Array_Resize` (`self.DummyV4`)))

(event `self.ReceiveTick`
  (params (DeltaSeconds :type "Float (single-precision)"))
  (`KismetSystemLibrary.PrintString` (`KismetStringLibrary.Conv_BoolToString` (`self.bUpdate`)) true true (struct :`G` 0.66 :`B` 1.0 :`A` 1.0) 0.0))

(event `DebugParticleData`
  (params (NiagaraSystemName :type String) (ParticleData :type "Array of GgNDI_BasicParticleData Structure"))
  (`KismetSystemLibrary.PrintString` (`KismetStringLibrary.Concat_StrStr` NiagaraSystemName " [ ArraySize : " (`KismetStringLibrary.Conv_IntToString` (`KismetArrayLibrary.Array_Length` ParticleData)) " ]") true true (struct :`R` 1.0 :`G` 0.5 :`B` 1.0 :`A` 1.0) 0.0))

(event `self.CustomReceiveParticleData`
  (params (Data :type "Array of GgNDI_BasicParticleData Structure (by ref)") (NiagaraSystem :type "NiagaraSystem Object Reference") (SimulationPositionOffset :type "Vector Structure (by ref)"))
  (bind _bparticleusageb (`self.bParticleUsageB`))
  (bind _ns_debrisb (`self.NS_DebrisB`))
  (bind _bparticleusageb_2 (`self.bParticleUsageB`))
  (bind _bparticleresetb (`self.bParticleResetB`))
  (bind _ns_debrisb_2 (`self.NS_DebrisB`))
  (bind _bparticlereseta (`self.bParticleResetA`))
  (bind _niagaracomponent (`NiagaraActor.NiagaraComponent` (`self.RefActorNSA`)))
  (bind _niagaracomponent_2 (`NiagaraActor.NiagaraComponent` (`self.RefActorNSA`)))
  (`self.DebugParticleData` (`KismetSystemLibrary.GetObjectName` NiagaraSystem) Data)
  (`|ExecutionSequence`
    (:`then_0`
      (if (== NiagaraSystem "/Game/PRJ/VFX/Debris/NS_DebrisA.NS_DebrisA")
        (bind _output_get (set `self.ParticleDataA` Data))
        (`|ExecutionSequence`
          (:`then_0`
            (for _array_element _output_get
              (bind (_uniqueid _mass _position) (break `GgNDI_BasicParticleData` _array_element))
              (if (<= (`KismetMathLibrary.Vector_Distance` (`self.K2_GetActorLocation`) _position) 1000.0)
                (for (_array_element_2 _array_index) _bparticleusageb_2
                  (if (not _array_element_2)
                    (`KismetArrayLibrary.Array_Set` _bparticleusageb_2 _array_index true)
                    (`KismetArrayLibrary.Array_Set` (`self.bParticleResetB`) _array_index true)
                    (`KismetArrayLibrary.Array_Set` (`self.ParticleDataToB`) _array_index _array_element)
                    (`KismetArrayLibrary.Array_Set` (`self.bParticleUsageA`) (`KismetMathLibrary.Round` _uniqueid))
                    (break))))))
          (:`then_1`
            (`NiagaraDataInterfaceArrayFunctionLibrary.SetNiagaraArrayBool` _niagaracomponent_2 "UseParticle" (`self.bParticleUsageA`) :!label _label)
            (`NiagaraDataInterfaceArrayFunctionLibrary.SetNiagaraArrayBool` _niagaracomponent_2 "ResetParticle" _bparticlereseta)
            (for (_array_element_3 _array_index_2) _bparticlereseta
              (if _array_element_3
                (`|ExecutionSequence`
                  (:`then_0`
                    (`KismetArrayLibrary.Array_Set` (`self.bParticleResetA`) _array_index_2))
                  (:`then_1`
                    (bind (_uniqueid_2 _mass_2 _position_2 _velocity _rotation) (break `GgNDI_BasicParticleData` (`|GetArrayItem` (`self.ParticleDataA`) _array_index_2)))
                    (`NiagaraDataInterfaceArrayFunctionLibrary.SetNiagaraArrayFloatValue` _niagaracomponent "InitMass" _array_index_2 _mass_2)
                    (`NiagaraDataInterfaceArrayFunctionLibrary.SetNiagaraArrayVectorValue` _niagaracomponent "InitPos" _array_index_2 _position_2)
                    (`NiagaraDataInterfaceArrayFunctionLibrary.SetNiagaraArrayVectorValue` _niagaracomponent "InitVel" _array_index_2 _velocity)
                    (`NiagaraDataInterfaceArrayFunctionLibrary.SetNiagaraArrayVector4Value` _niagaracomponent "InitRot" _array_index_2 _rotation)))))
            (`NiagaraDataInterfaceArrayFunctionLibrary.SetNiagaraArrayBool` _ns_debrisb "UseParticle" (`self.bParticleUsageB`))
            (`NiagaraDataInterfaceArrayFunctionLibrary.SetNiagaraArrayBool` _ns_debrisb "ResetParticle" _bparticleresetb)
            (for (_array_element_4 _array_index_3) _bparticleresetb
              (if _array_element_4
                (`|ExecutionSequence`
                  (:`then_0`
                    (`KismetArrayLibrary.Array_Set` (`self.bParticleResetB`) _array_index_3))
                  (:`then_1`
                    (bind (_uniqueid_3 _mass_3 _position_3 _velocity_2 _rotation_2) (break `GgNDI_BasicParticleData` (`|GetArrayItem` (`self.ParticleDataToB`) _array_index_3)))
                    (`NiagaraDataInterfaceArrayFunctionLibrary.SetNiagaraArrayFloatValue` _ns_debrisb_2 "InitMass" _array_index_3 _mass_3)
                    (`NiagaraDataInterfaceArrayFunctionLibrary.SetNiagaraArrayVectorValue` _ns_debrisb_2 "InitPos" _array_index_3 _position_3)
                    (`NiagaraDataInterfaceArrayFunctionLibrary.SetNiagaraArrayVectorValue` _ns_debrisb_2 "InitVel" _array_index_3 _velocity_2)
                    (`NiagaraDataInterfaceArrayFunctionLibrary.SetNiagaraArrayVector4Value` _ns_debrisb_2 "InitRot" _array_index_3 _rotation_2)))))))))
    (:`then_1`
      (if (== NiagaraSystem "/Game/PRJ/VFX/Debris/NS_DebrisB1.NS_DebrisB1")
        (`|ExecutionSequence`
          (:`then_0`
            (for _array_element_5 Data
              (bind (_uniqueid_4 _mass_4 _position_4) (break `GgNDI_BasicParticleData` _array_element_5))
              (if (> (`KismetMathLibrary.Vector_Distance` (`self.K2_GetActorLocation`) _position_4) 1000.0)
                (bind _returnvalue (`KismetMathLibrary.Round` _uniqueid_4))
                (if (`|GetArrayItem` _bparticleusageb _returnvalue)
                  (`KismetArrayLibrary.Array_Set` _bparticleusageb _returnvalue)
                  (bind _returnvalue_2 (`KismetMathLibrary.Round` (`.UniqueID` (break `GgNDI_BasicParticleData` (`|GetArrayItem` (`self.ParticleDataToB`) _returnvalue)))))
                  (`KismetArrayLibrary.Array_Set` (`self.bParticleResetA`) _returnvalue_2 true)
                  (`KismetArrayLibrary.Array_Set` (`self.ParticleDataA`) _returnvalue_2 _array_element_5)
                  (`KismetArrayLibrary.Array_Set` (`self.bParticleUsageA`) _returnvalue_2 true)))))
          (:`then_1`
            (goto _label)))))))

(fn `UserConstructionScript`)