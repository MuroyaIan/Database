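; BP_RotateLight is a light Blueprint that swings its Cube component back and forth on the pitch axis between two configurable angles.
; Tick feeds delta time into the ライトの回転処理 graph, which accumulates time over each swing's duration.
; UpdateRotation applies an ease-in-out lerp to Cube's relative rotation.
; After each swing, it swaps the start and end angles and uses a Wait-gated Delay to pause before reversing.
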(event `self.ReceiveTick`
  (params (DeltaSeconds :type "Float (single-precision)"))
  (bind _output_get (set `self.DeltaSec` DeltaSeconds))
  (`|ExecutionSequence`
    (:`then_0`
      (if (`self.bWait`)
        (`KismetSystemLibrary.Delay` (`self.往復の間隔（秒）`))
        (set `self.bWait` false))
      (bind _output_get_2 (set `self.CalcTime` (+ (`self.CalcTime`) _output_get)))
      (bind _returnvalue (/ _output_get_2 (`self.揺れ時間（一回/秒）`)))
      (if (>= _returnvalue 1.0)
        (set `self.CalcTime` 0.0)
        (set `self.DeltaSec` (`self.揺れ始めの角度（度）`))
        (set `self.揺れ始めの角度（度）` (`self.揺れ終了の角度（度）`))
        (set `self.揺れ終了の角度（度）` (`self.DeltaSec`))
        (set `self.bWait` true)
        (else
          (`self.UpdateRotation` _returnvalue))))))

(fn `UpdateRotation`
  (params (Alpha :type "Float (double-precision) (by ref)"))
  (`SceneComponent.K2_SetRelativeRotation` (`self.Cube`) (`KismetMathLibrary.MakeRotator` 0.0 (`KismetMathLibrary.Lerp` (`self.揺れ始めの角度（度）`) (`self.揺れ終了の角度（度）`) (`|EaseFunction` "EaseInOut" Alpha 0.0 1.0 2.0))) false false))

(fn `UserConstructionScript`)